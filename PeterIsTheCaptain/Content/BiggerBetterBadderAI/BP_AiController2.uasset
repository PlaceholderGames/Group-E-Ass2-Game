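; AI controller that runs the AIBT behavior tree when it possesses an AI pawn and tracks whether it can see the player.
; Its AIPerception updates set the CanSeePlayer blackboard bool from whether the stimulus was sensed.
; Any PaperCharacter counts as the player, as the only filter is a cast to that class.
; Debug strings print when the target is sensed or lost.
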(event `self.OnPossess`
  (params (PossessedPawn :type "Pawn Object Reference"))
  (cast `/Game/BiggerBetterBadderAI/AI` PossessedPawn)
  (`self.RunBehaviorTree` "/Game/BiggerBetterBadderAI/AIBT.AIBT"))

(event `self.AIPerception.OnTargetPerceptionUpdated`
  (params (Actor :type "Actor Object Reference") (Stimulus :type "AIStimulus Structure"))
  (bind (_age _expirationage _strength _stimuluslocation _receiverlocation _tag _bsuccessfullysensed) (break `AIStimulus` Stimulus))
  (cast `PaperCharacter` Actor)
  (`BlackboardComponent.SetValueAsBool` (`AIBlueprintHelperLibrary.GetBlackboard` null) "CanSeePlayer" _bsuccessfullysensed)
  (if _bsuccessfullysensed
    (`KismetSystemLibrary.PrintString` "I see you")
    (else
      (`KismetSystemLibrary.PrintString` "Where did you go?"))))

(fn `UserConstructionScript`)