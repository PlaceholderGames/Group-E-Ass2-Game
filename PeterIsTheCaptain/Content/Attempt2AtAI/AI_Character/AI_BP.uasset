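; AI_BP is a Paper2D guard character that ends the run when the player character, Jon, touches it.
; Overlapping its Box disables Jon's input, prints a red death message and, after a short delay, opens Map1.
; A custom UpdateAnimation event, not called within this file, picks the walking or idle flipbook from a zero-rotation forward vector's length, so it always selects walking.
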(event `self.Box.OnComponentBeginOverlap`
  (params (OverlappedComponent :type "PrimitiveComponent Object Reference") (OtherActor :type "Actor Object Reference") (OtherComp :type "PrimitiveComponent Object Reference") (OtherBodyIndex :type Integer) (bFromSweep :type Boolean) (SweepResult :type "HitResult Structure (by ref)"))
  (bind _asjon (cast `/Game/2Dcharacter/Jon` OtherActor))
  (`self.DisableInput` _asjon null)
  (`KismetSystemLibrary.PrintString` "You have dead" true true (struct :`R` 1.0 :`A` 1.0) 4.0)
  (`KismetSystemLibrary.Delay` 3.0)
  (`GameplayStatics.OpenLevel` "Map1"))

(event `Update Animation`
  (`PaperFlipbookComponent.SetFlipbook` (`self.Sprite`) (select `bool` (> (`KismetMathLibrary.VSize` (`KismetMathLibrary.GetForwardVector` (struct))) 0.0) :`false` "/Game/Sprites/Guard1/Guard1_Idle.Guard1_Idle" :`true` "/Game/Sprites/Guard1/Guard1_Walking.Guard1_Walking" :!type "PaperFlipbook Object Reference")))

(fn `UserConstructionScript`)