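; Clickable pickup actor that adds an item to the player's inventory.
; The construction script picks the static mesh from a mesh array using the item index.
; Clicking the mesh finds the first top-level Inventory widget, passes it the index through Additem, and destroys the actor.
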(event `self.StaticMesh.OnClicked`
  (params (TouchedComponent :type "PrimitiveComponent Object Reference") (ButtonPressed :type "Key Structure" :default "AnyKey"))
  (bind _foundwidgets (`WidgetBlueprintLibrary.GetAllWidgetsOfClass` "/Game/Blueprints/Inventroy/Inventory.Inventory_C"))
  (`/Game/Blueprints/Inventroy/Inventory.additem` (cast `/Game/Blueprints/Inventroy/Inventory` (`|GetArrayItem` _foundwidgets) :!pure true) (`self.index`))
  (`self.K2_DestroyActor`))

(fn `UserConstructionScript`
  (`StaticMeshComponent.SetStaticMesh` (`self.StaticMesh`) (`|GetArrayItem` (`self.meshes`) (`self.index`))))