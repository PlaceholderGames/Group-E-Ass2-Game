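; AI controller for the AI_BP guard character, driving it through the AI_BT behavior tree.
; On BeginPlay it sets a slow walk speed, starts the tree and copies the pawn's four guard points into the blackboard.
; When pawn sensing sees a pawn, it stores it as the blackboard Target and raises the walk speed, with no logic here to clear the target or slow down again.
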(event `self.ReceiveBeginPlay`
  (bind _asai_bp (cast `/Game/Attempt2AtAI/AI_Character/AI_BP` (`self.K2_GetPawn`)))
  (set `CharacterMovementComponent.MaxWalkSpeed` 150.0 (`Character.CharacterMovement` _asai_bp))
  (`self.RunBehaviorTree` "/Game/Attempt2AtAI/AI_BRAIN/AI_BT.AI_BT")
  (bind _asai_bp_2 (cast `/Game/Attempt2AtAI/AI_Character/AI_BP` (`self.K2_GetPawn`)))
  (`BlackboardComponent.SetValueAsObject` (`AIBlueprintHelperLibrary.GetBlackboard` self) "guardpoint1" (`/Game/Attempt2AtAI/AI_Character/AI_BP.GuardPoint1` _asai_bp_2))
  (`BlackboardComponent.SetValueAsObject` (`AIBlueprintHelperLibrary.GetBlackboard` self) "guardpoint2" (`/Game/Attempt2AtAI/AI_Character/AI_BP.GuardPoint2` _asai_bp_2))
  (`BlackboardComponent.SetValueAsObject` (`AIBlueprintHelperLibrary.GetBlackboard` self) "guardpoint3" (`/Game/Attempt2AtAI/AI_Character/AI_BP.GuardPoint3` _asai_bp_2))
  (`BlackboardComponent.SetValueAsObject` (`AIBlueprintHelperLibrary.GetBlackboard` self) "guardpoint4" (`/Game/Attempt2AtAI/AI_Character/AI_BP.GuardPoint4` _asai_bp_2)))

(event `self.PawnSensing.OnSeePawn`
  (params (Pawn :type "Pawn Object Reference"))
  (`BlackboardComponent.SetValueAsObject` (`AIBlueprintHelperLibrary.GetBlackboard` self) "Target" Pawn)
  (bind _asai_bp (cast `/Game/Attempt2AtAI/AI_Character/AI_BP` (`self.K2_GetPawn`)))
  (set `CharacterMovementComponent.MaxWalkSpeed` 250.0 (`Character.CharacterMovement` _asai_bp)))

(fn `UserConstructionScript`)