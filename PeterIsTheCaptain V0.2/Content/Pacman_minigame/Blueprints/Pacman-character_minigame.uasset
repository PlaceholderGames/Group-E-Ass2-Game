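; Player character for the Pacman minigame, moved by two input axes and tracking how many edibles it has eaten.
; The axes feed movement input along world Z for up/down and world X for left/right.
; Overlapping an Edibles actor increments a counter, which is printed until it reaches a hardcoded total that opens the World level.
; The Set My Flipbook function is an empty stub.
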(event `InputAxis|NewAxisMapping_1Pacman_minigame_movement-UpDown`
  (params (AxisValue :type "Float (single-precision)"))
  ;[1 1 1] Character movement Up and Down
  (`self.AddMovementInput` (0.0 0.0 1.0) AxisValue))

(event `InputAxis|NewAxisMapping_2Pacman_minigame_movement-LeftRight`
  (params (AxisValue :type "Float (single-precision)"))
  ;[1 1 1] Character Movement Left and Right
  (`self.AddMovementInput` (1.0 0.0 0.0) AxisValue))

(event `self.ReceiveActorBeginOverlap`
  (params (OtherActor :type "Actor Object Reference"))
  ;[1 1 1] Edibles counter, eating all of them opens World Level
  (cast `/Game/Pacman_minigame/Blueprints/Edibles` OtherActor)
  (bind _output_get (set `self.EdiblesEaten` (+ (`self.EdiblesEaten`) 1)))
  (if (>= _output_get 105)
    (`GameplayStatics.OpenLevel` "World")
    (else
      (`KismetSystemLibrary.PrintString` (`KismetStringLibrary.Conv_IntToString` (`self.EdiblesEaten`))))))

(fn `Set My Flipbook`)

(fn `UserConstructionScript`)