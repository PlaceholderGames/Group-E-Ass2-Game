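; Base inventory Blueprint that stores picked-up item actors as slots in ItemList, limited by total weight.
; AddItemToInventory sends stackable items to HasPartialStack, which matches name and MaxStackSize below zero, and otherwise adds a slot if HasInventorySpace passes.
; Stored items get a fixed slot count increment and their actor is destroyed.
; The resulting slot index overwrites MaxWeight, the same variable used as the weight limit.
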(fn `AddItemToInventory`
  (params (Target :type "/Game/Blueprints/Inventory/BaseItem Object Reference"))
  (returns (MaxWeight :type Integer))
  (bind _maxweight (`self.MaxWeight`))
  (`self.CanItStack` Target
    (:`true`
      (bind _index (`self.HasPartialStack` Target)
        (:`true`
          (set `self.MaxWeight` _index))
        (:`false`
          (`self.HasInventorySpace` :!label _label
            (:`true`
              (bind _returnvalue (`KismetArrayLibrary.Array_Add` (`self.ItemList`) (make `/Game/Blueprints/Inventory/InventorySLot` Target 10)))
              (set `self.MaxWeight` _returnvalue)
              (`self.K2_DestroyActor` Target))))))
    (:`false`
      (goto _label)))
  (`KismetSystemLibrary.PrintString` (`KismetStringLibrary.BuildString_Int` "" "" _maxweight))
  (return _maxweight))

(fn `UserConstructionScript`)